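; Food pickup actor for a food game that adds or removes player points depending on its type (DruhJidla): donut, pizza, carrot or bottle.
; The construction script selects the mesh and score from that type, with donut and pizza negative, carrot and bottle positive.
; On Interacted, it passes the score to BP_ThirdPersonCharacter's PridatBod and destroys itself.
; Pizza also disables player input for a short delay before destruction.
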(event `PickUP event`
  (params (Object :type "Actor Object Reference")))

(event `/Game/BP/Interfaces/Interaction_Interface.Interacted`
  (bind _returnvalue (`GameplayStatics.GetPlayerController` 0))
  (bind _returnvalue_2 (`GameplayStatics.GetPlayerCharacter` 0))
  (`self.pickUP` _returnvalue_2)
  (if (`|EnumEquality` (`self.druhJidla`) "NewEnumerator1")
    (`self.DisableInput` _returnvalue_2 _returnvalue)
    (`KismetSystemLibrary.Delay` 2.0)
    (`self.EnableInput` _returnvalue_2 _returnvalue)
    (`self.K2_DestroyActor`)
    (else
      (`self.K2_DestroyActor`))))

(fn `pickUP`
  (params (Object :type "Actor Object Reference"))
  (bind _asbp_third_person_character (cast `/Game/ThirdPerson/Blueprints/BP_ThirdPersonCharacter` Object))
  (`/Game/ThirdPerson/Blueprints/BP_ThirdPersonCharacter.pridatBod` _asbp_third_person_character (`self.skore`)))

(fn `UserConstructionScript`
  (`StaticMeshComponent.SetStaticMesh` (`self.StaticMesh`) (select `/Game/BP/druhyJidel` (`self.druhJidla`) :`NewEnumerator0` "/Game/models/jidlohra_donut.jidlohra_donut" :`NewEnumerator1` "/Game/models/jidlohra_pizza.jidlohra_pizza" :`NewEnumerator2` "/Game/models/jidlohra_mrkev.jidlohra_mrkev" :`NewEnumerator3` "/Game/models/jidlohra_lahev.jidlohra_lahev" :!type "StaticMesh Object Reference"))
  (set `self.skore` (select `/Game/BP/druhyJidel` (`self.druhJidla`) :`NewEnumerator0` -1 :`NewEnumerator1` -2 :`NewEnumerator2` 2 :`NewEnumerator3` 1)))